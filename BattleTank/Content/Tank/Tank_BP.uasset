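; Tank_BP is the player-controlled tank pawn, translating input into track throttle, camera aiming and firing.
; On BeginPlay it passes its turret, barrel and track components to inherited setters.
; Each track takes its own throttle axis for differential steering, and Fire triggers on the fire action.
; Aim axes orbit the camera, yawing a horizontal gimbal and pitching the spring arm at frame-rate-independent rates.
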(event EventBeginPlay
  (Class|Tank|SetTurretReference (Variables|Default|GetTurret))
  (Class|Tank|SetBarrelReference (Variables|Default|GetBarrel))
  (Class|Tank|SetLeftTrackReference (Variables|Default|GetLeft%20Track))
  (Class|Tank|SetRightTrackReference (Variables|Default|GetRight%20Track)))

(event Input|ActionEvents|InputActionFire
  (params (Key :type Key%20Structure :default "AnyKey"))
  ;[1 1 1] CameraInputBinding
  (:Pressed
    (Class|Tank|Fire)))

(event Input|AxisEvents|InputAxisLeftTrackThrottle
  (params (AxisValue :type Float%20%28single-precision%29))
  ;[1 1 1] MovementSection
  (Class|TankTrack|SetThrottle (Variables|Default|GetLeft%20Track) AxisValue))

(event Input|AxisEvents|InputAxisRightTrackThrottle
  (params (AxisValue :type Float%20%28single-precision%29))
  ;[1 1 1] MovementSection
  (Class|TankTrack|SetThrottle (Variables|Default|GetRight%20Track) AxisValue))

(event Input|AxisEvents|InputAxisAimVertically
  (params (AxisValue :type Float%20%28single-precision%29))
  ;[1 1 1] CameraInputBinding
  (Transformation|AddLocalRotation (Variables|Default|GetSpringArm) (Math|Rotator|MakeRotator 0.0 (* AxisValue (Utilities|Time|GetWorldDeltaSeconds) 5e+01) 0.0) false false))

(event Input|AxisEvents|InputAxisAimHorizontally
  (params (AxisValue :type Float%20%28single-precision%29))
  ;[1 1 1] CameraInputBinding
  (Transformation|AddLocalRotation (Variables|Default|GetHorizontalGimbal) (Math|Rotator|MakeRotator 0.0 0.0 (* AxisValue (Utilities|Time|GetWorldDeltaSeconds) 1e+02)) false false))

(fn ConstructionScript)